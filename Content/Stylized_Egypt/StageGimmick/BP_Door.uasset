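; BP_Door is an automatic double sliding door stage gimmick that opens when a BP_PC enters its Box trigger and closes when it leaves.
; Overlap begin plays a timeline, and overlap end reverses it.
; The timeline's alpha feeds an EaseInOut that slides AutoDoor and AutoDoor1 along relative Y from InitialLocation toward opposite-signed NewLoacation offsets.
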(event `self.Box.OnComponentBeginOverlap`
  (params (OverlappedComponent :type "PrimitiveComponent Object Reference") (OtherActor :type "Actor Object Reference") (OtherComp :type "PrimitiveComponent Object Reference") (OtherBodyIndex :type Integer) (bFromSweep :type Boolean) (SweepResult :type "HitResult Structure (by ref)"))
  (bind _initiallocation (`self.InitialLocation`))
  (bind _newloacation (`self.NewLoacation`))
  (cast `/Game/BP/Character/BP_PC` OtherActor)
  (bind (_direction _alpha) (`Timeline|タイムライン_0` :!label _label)
    (:`Update`
      (`SceneComponent.K2_SetRelativeLocation` (`self.AutoDoor`) (`KismetMathLibrary.MakeVector` 0.0 (`|EaseFunction` "EaseInOut" _alpha _initiallocation (* _newloacation -1.0))) false false)
      (`SceneComponent.K2_SetRelativeLocation` (`self.AutoDoor1`) (`KismetMathLibrary.MakeVector` 0.0 (`|EaseFunction` "EaseInOut" _alpha _initiallocation _newloacation)) false false))))

(event `self.Box.OnComponentEndOverlap`
  (params (OverlappedComponent :type "PrimitiveComponent Object Reference") (OtherActor :type "Actor Object Reference") (OtherComp :type "PrimitiveComponent Object Reference") (OtherBodyIndex :type Integer))
  (cast `/Game/BP/Character/BP_PC` OtherActor)
  (goto _label :!via `Reverse`))

(fn `NewFunction_0`
  (set `self.AutoDoor1` null))

(fn `UserConstructionScript`)