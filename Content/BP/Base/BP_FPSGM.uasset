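; Game mode for an FPS that assigns players to two teams and handles their respawn.
; On login, an incrementing counter sets each player state's ID, and its parity sets the team.
; RespawnPlayer waits, spawns a BP_PC at the given location and possesses it with the controller indexed by SpawnID.
; BeginPlay starts a looping one-second timer, but its handler is empty and the countdown logic is disconnected.
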(event `Clock_SoundFPS`)

(event `self.ReceiveBeginPlay`
  (`self.Start`))

(event `self.K2_PostLogin`
  (params (NewPlayer :type "PlayerController Object Reference"))
  (bind _asbp_player_state (cast `/Game/BP/Character/BP_PlayerState` (`Controller.PlayerState` NewPlayer)))
  (bind _result (`/Engine/EditorBlueprintResources/StandardMacros.IncrementInt` (`self.Next_Teame_ID`))
    (:`  `
      (bind _output_get (set `self.Next_Teame_ID` _result))
      (set `/Game/BP/Character/BP_PlayerState.MyID` _output_get _asbp_player_state)
      (bind _output_get_2 (set `/Game/BP/Character/BP_PlayerState.TeamID` (mod _output_get 2) _asbp_player_state))
      (switch `int` _output_get_2))))

(event `self.K2_OnRestartPlayer`
  (params (NewPlayer :type "Controller Object Reference")))

(event `Respawn Player`
  (params (`Used Contoller` :type "PlayerController Object Reference") (StartLocation :type "Vector Structure") (SpawnID :type Integer))
  (`KismetSystemLibrary.Delay` 5.0)
  (bind _returnvalue (`|SpawnActorFromClass` "/Game/BP/Character/BP_PC.BP_PC_C" (`KismetMathLibrary.Conv_VectorToTransform` StartLocation) "AdjustIfPossibleButAlwaysSpawn" "OverrideRootScale" `Used Contoller` null))
  (`Controller.Possess` (`GameplayStatics.GetPlayerController` (- SpawnID 1)) _returnvalue))

(fn `NewFunction_0`
  (params (self2 :type "Controller Object Reference"))
  (bind _asbp_player_state (cast `/Game/BP/Character/BP_PlayerState` (`Controller.PlayerState` self2)))
  (bind _result (`/Engine/EditorBlueprintResources/StandardMacros.IncrementInt` (`/Game/BP/Character/BP_PlayerState.MyID` _asbp_player_state))
    (:`  `
      (bind _output_get (set `/Game/BP/Character/BP_PlayerState.MyID` _result _asbp_player_state))
      (bind _output_get_2 (set `/Game/BP/Character/BP_PlayerState.TeamID` (mod _output_get 2) _asbp_player_state))
      (switch `int` _output_get_2))))

(fn `UserConstructionScript`)