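; FPS game state Blueprint that runs a 30-second countdown and flags when it ends.
; BeginPlay calls Start, which sets Time and starts a looping one-second timer on Clock_SoundFPS by function name.
; Each tick of that timer decrements Time; at zero it sets CheckTimer to true and clears the timer.
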(event `Clock_SoundFPS`
  (set `self.Time` (- (`self.Time`) 1))
  (if (== (`self.Time`) 0)
    (set `self.CheckTimer` true)
    (`KismetSystemLibrary.K2_ClearTimer` null "Clock_SoundFPS")))

(event `self.ReceiveBeginPlay`
  (`self.Start`))

(fn `UserConstructionScript`)