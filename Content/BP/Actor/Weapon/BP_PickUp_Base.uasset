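; Base weapon pickup actor that lets the player interact to receive a weapon while standing inside its sphere.
; Sphere overlap binds the pickup event to the player's interact input and shows the pickup HUD; leaving unbinds it and removes the HUD.
; The pickup event passes weapon class, weapon type and bullet type to PickUpSpawnWeapon on the player 0 pawn cached at BeginPlay.
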(event `self.ReceiveBeginPlay`
  (bind _asbp_pc (cast `/Game/BP/Character/BP_PC` (`GameplayStatics.GetPlayerPawn` 0)))
  (set `self.As BP PC` _asbp_pc))

(event `self.Sphere.OnComponentBeginOverlap`
  (params (OverlappedComponent :type "PrimitiveComponent Object Reference") (OtherActor :type "Actor Object Reference") (OtherComp :type "PrimitiveComponent Object Reference") (OtherBodyIndex :type Integer) (bFromSweep :type Boolean) (SweepResult :type "HitResult Structure (by ref)"))
  (bind _asbp_pc (cast `/Game/BP/Character/BP_PC` OtherActor))
  (add `/Game/BP/Character/BP_PC.Interact` _asbp_pc (delegate `PickUpEvent`))
  (bind _pickup_hud (`/Game/BP/Character/BP_PC.PickUp_HUD` _asbp_pc))
  (if (not (`Widget.IsInViewport` _pickup_hud))
    (`UserWidget.AddToViewport` _pickup_hud 0)))

(event `PickUpEvent`
  (`/Game/BP/Character/BP_PC.PickUp_SpawnWeapon` (`self.As BP PC`) (`self.Weapon_Class`) (`self.WeaponType`) (`self.BulletType`)))

(event `self.Sphere.OnComponentEndOverlap`
  (params (OverlappedComponent :type "PrimitiveComponent Object Reference") (OtherActor :type "Actor Object Reference") (OtherComp :type "PrimitiveComponent Object Reference") (OtherBodyIndex :type Integer))
  (bind _asbp_pc (cast `/Game/BP/Character/BP_PC` OtherActor))
  (remove `/Game/BP/Character/BP_PC.Interact` _asbp_pc (delegate `PickUpEvent`))
  (`Widget.RemoveFromParent` (`/Game/BP/Character/BP_PC.PickUp_HUD` _asbp_pc)))

(fn `UserConstructionScript`)