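; BP_Audio_Weapon is the auditory weapon actor that fires sound bullets.
; Its SpawnAudioBullet function always spawns a BP_Audio_Bullet at the weapon mesh's Muzzle socket, oriented along the mesh's forward vector.
; It then sets itself as the bullet's Weapon and returns the bullet to the caller.
; The event graph is empty, construction only calls the parent, and a gunshot sound node is left unconnected.
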(fn `Spawn_Audio_Bullet`
  (returns (Audio_Bullet :type "/Game/BP/Actor/Weapon/Bullets/AudioVisual_Bullets/BP_Audio_Bullet Object Reference"))
  (bind _weaponmesh (`self.WeaponMesh`))
  (bind _returnvalue_location (`KismetMathLibrary.BreakTransform` (`SceneComponent.GetSocketTransform` _weaponmesh "Muzzle" "RTS_World")))
  ;[0.1375 0.009595 1] 聴覚：音弾
  (bind _returnvalue (`|SpawnActorFromClass` "/Game/BP/Actor/Weapon/Bullets/AudioVisual_Bullets/BP_Audio_Bullet.BP_Audio_Bullet_C" (`KismetMathLibrary.MakeTransform` _returnvalue_location (`KismetMathLibrary.Conv_VectorToRotator` (`SceneComponent.GetForwardVector` _weaponmesh))) "AlwaysSpawn" "OverrideRootScale" null null)) ; 弾の生成( 実体を生成してからじゃないと数値を設定できない )
  (set `/Game/BP/Actor/Weapon/Bullets/AudioVisual_Bullets/BP_Audio_Bullet.Weapon` self _returnvalue)
  (return _returnvalue))

(fn `UserConstructionScript`
  (`parent.UserConstructionScript`))