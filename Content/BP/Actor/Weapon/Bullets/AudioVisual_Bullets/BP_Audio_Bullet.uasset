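; BP_Audio_Bullet is a chargeable sound projectile that starts silent, with collision disabled.
; While charging, Tick pins the bullet to the weapon's Muzzle socket transform.
; ChangeTheBullet grows its scale toward a maximum, updating volume and damage through the weapon reference as it grows.
; BulletAfterChange releases it: tracking stops, projectile movement and collision turn on, and audio plays at the weapon's accumulated volume, which then resets.
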(event `self.ReceiveBeginPlay`
  (`parent.ReceiveBeginPlay`)
  (set `ProjectileMovementComponent.bSimulationEnabled` (`self.Accuser`) (`self.ProjectileMovement`)) ; 弾の動きを止める
  (`self.SetActorEnableCollision` false) ; 当たり判定を無効
  (`AudioComponent.Stop` (`self.Audio`)) ; 音を止める
)

(event `self.ReceiveTick`
  (params (DeltaSeconds :type "Float (single-precision)"))
  (bind (_returnvalue_location _returnvalue_rotation) (`KismetMathLibrary.BreakTransform` (`SceneComponent.GetSocketTransform` (`/Game/BP/Actor/Weapon/BP_Weapon_Base.WeaponMesh` (`self.Weapon`)) "Muzzle" "RTS_World")))
  (`parent.ReceiveTick` DeltaSeconds)
  (if (`self.LocationChange`)
    (`SceneComponent.K2_SetRelativeTransform` (`self.Bullet`) (`KismetMathLibrary.MakeTransform` _returnvalue_location _returnvalue_rotation (`self.scale`)) false false) ; 弾が銃の位置に追跡
  ))

(fn `Bullet_After_Change`
  (bind _audio (`self.Audio`))
  (bind _weapon (`self.Weapon`))
  (set `self.LocationChange` false) ; 弾が銃の位置に追跡状態OFF
  (set `ProjectileMovementComponent.bSimulationEnabled` true (`self.ProjectileMovement`)) ; 弾が動き出す
  (`AudioComponent.SetVolumeMultiplier` _audio (`/Game/BP/Actor/Weapon/BP_Weapon_Base.bullet_volume` _weapon)) ; 音を設定
  (`self.SetActorEnableCollision` true) ; 当たり判定の復活
  (`AudioComponent.Play` _audio 0.0) ; 音を鳴らす
  (set `/Game/BP/Actor/Weapon/BP_Weapon_Base.bullet_volume` 0.0 _weapon))

(fn `Change_The_Bullet`
  (bind _weapon (`self.Weapon`))
  ;[1 1 1] 弾を変化させる処理
  (set `self.LocationChange` true) ; 弾が銃の位置に追跡状態ON
  (if (`KismetMathLibrary.NotEqualExactly_VectorVector` (`self.scale`) (`self.Max_Scale`))
    (bind _output_get (set `self.scale` (`self.scale`)))
    (bind _output_get_2 (set `self.scale` _output_get))
    (set `self.scale` (+ _output_get_2 (`self.+_scale`)))
    (`/Game/BP/Actor/Weapon/BP_Weapon_Base.Vollume` _weapon) ; 弾の音量
    (`self.Damage` (`/Game/BP/Actor/Weapon/BP_Weapon_Base.Bullet_Damage` _weapon)) ; 弾のダメージ量
    (else
      (set `self.scale` (`self.scale`)))))

(fn `UserConstructionScript`
  (`parent.UserConstructionScript`))