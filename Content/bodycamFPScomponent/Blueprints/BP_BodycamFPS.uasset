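; Player character for a bodycam-style FPS, handling movement, jump, sprint, free aim, pistol fire and reload.
; Mouse input drives free-aim and camera shake/vignette components, with view pitch limited at BeginPlay.
; The free-aim transform and clamped pitch rotation are computed on authority or local control, then sent through RPCs.
; Sprint toggles walk speed via server-to-client events; fire and reload RPCs play arm montages and weapon animations.
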(event `self.ReceiveBeginPlay`
  (bind _returnvalue (`GameplayStatics.GetPlayerCameraManager` 0))
  ;[1 1 1] イベント開始再生
  (set `PlayerCameraManager.ViewPitchMax` 35.0 _returnvalue)
  (set `PlayerCameraManager.ViewPitchMin` -45.0 _returnvalue))

(event `InputAxis|LookUp` :overrideparent false
  (params (AxisValue :type "Float (single-precision)"))
  ;[1 1 1] エイムスペース
  (`self.AddControllerPitchInput` AxisValue)
  (if (!= AxisValue 0.0)
    (`|ExecutionSequence`
      (:`then_0`
        (`self.AimRot`)
        (`self.RPC_SkeRot` (`self.ControlRot_Rep`)))
      (:`then_1`
        (`self.MouseMoves`)))))

(event `RPC_SkeRot`
  (params (ControlRot_Rep :type "Rotator Structure"))
  ;[1 1 1] エイムスペース
  (set `self.ControlRot_Rep` ControlRot_Rep))

(event `InputAxis|MoveForward` :overrideparent false
  (params (AxisValue :type "Float (single-precision)"))
  ;[1 1 1] 動きの入力
  (`self.AddMovementInput` (`KismetMathLibrary.GetForwardVector` (`KismetMathLibrary.MakeRotator` 0.0 0.0 (.yaw (`self.GetControlRotation`)))) AxisValue))

(event `Key|LeftShift`
  (params (Key :type "Key Structure"))
  ;[1 1 1] スプリント
  (:`Pressed`
    (`self.SprintOnServer` true))
  (:`Released`
    (`self.SprintOnServer` false)))

(event `MouseMoves`
  (bind _camera (`self.Camera`))
  ;[1 1 1] フリーエイム(複製)
  (`|ExecutionSequence`
    (:`then_0`
      (if (or (`self.HasAuthority`) (`self.IsLocallyControlled`))
        (bind _freeaimtransform (`/Game/bodycamFPScomponent/Blueprints/BP_AC_FreeAim.FreeAimComponent` (`self.BP_AC_FreeAim`) (`self.Sphere`) (`self.GetInputAxisValue`) (`self.GetInputAxisValue`) 1.0 true))
        (bind _output_get (set `self.Free Aim Transform` _freeaimtransform))
        (`self.RPCFreeAim` _output_get)))
    (:`then_1`
      ;[1 1 1] プレイヤーのカメラ（複製は不要）
      (`/Game/bodycamFPScomponent/Blueprints/BP_AC_Camera.Camera Shake & Vignette` (`self.BP_AC_Camera`) _camera (`self.GetVelocity`) (`SceneComponent.K2_GetComponentRotation` _camera) false false true))))

(event `InputAxis|Turn` :overrideparent false
  (params (AxisValue :type "Float (single-precision)"))
  ;[1 1 1] マウス入力
  (`self.AddControllerYawInput` AxisValue)
  (`self.MouseMoves`))

(event `SprintOnServer`
  (params (Sprinting :type Boolean))
  ;[1 1 1] スプリント
  (`self.SprintOnClient` Sprinting))

(event `RPCFreeAim`
  (params (`Free Aim Transform` :type "Transform Structure"))
  ;[1 1 1] フリーエイム(複製)
  (bind _output_get (set `self.Free Aim Transform` `Free Aim Transform`))
  (`self.MulticastFreeAim` _output_get))

(event `InputAxis|MoveRight` :overrideparent false
  (params (AxisValue :type "Float (single-precision)"))
  ;[1 1 1] 動きの入力
  (`self.AddMovementInput` (`KismetMathLibrary.GetRightVector` (`KismetMathLibrary.MakeRotator` 0.0 0.0 (.yaw (`self.GetControlRotation`)))) AxisValue))

(event `InputAction|Jump` :overrideparent false
  (params (Key :type "Key Structure"))
  ;[1 1 1] ジャンプ
  (:`Pressed`
    (`self.Jump`))
  (:`Released`
    (`self.StopJumping`)))

(event `SprintOnClient`
  (params (`Sprinting?` :type Boolean))
  (bind _charactermovement (`self.CharacterMovement`))
  ;[1 1 1] スプリント
  (if `Sprinting?`
    (set `CharacterMovementComponent.MaxWalkSpeed` 600.0 _charactermovement)
    (else
      (set `CharacterMovementComponent.MaxWalkSpeed` 150.0 _charactermovement))))

(event `MulticastFreeAim`
  (params (`Free Aim Transform` :type "Transform Structure"))
  ;[1 1 1] フリーエイム(複製)
  (set `self.Free Aim Transform` `Free Aim Transform`))

(event `Key|R`
  (params (Key :type "Key Structure"))
  ;[1 1 1] リロード
  (:`Pressed`
    (`self.RPC_PlayReloadAnimation`)))

(event `Key|LeftMouseButton`
  (params (Key :type "Key Structure"))
  ;[1 1 1] ファイアロジック
  (:`Pressed`
    (`self.RPC_FireAnimation`)))

(event `RPC_PlayReloadAnimation`
  ;[1 1 1] リロード
  (`self.PlayReloadAnimation`))

(event `RPC_FireAnimation`
  ;[1 1 1] ファイアロジック
  (`self.PlayFireAnimation`))

(event `PlayReloadAnimation`
  ;[1 1 1] リロード
  (`|PlayMontage` (`self.Mesh`) "/Game/bodycamFPScomponent/Demo/Character/Anims/Anim_Arms_Pistol_Reload_Montage.Anim_Arms_Pistol_Reload_Montage"
    (:`then`
      (`SkeletalMeshComponent.PlayAnimation` (`self.Weapon`) "/Game/bodycamFPScomponent/Demo/Character/Anims/Anim_Pistol_Reload.Anim_Pistol_Reload" false))))

(event `PlayFireAnimation`
  ;[1 1 1] ファイアロジック
  (`|PlayMontage` (`self.Mesh`) "/Game/bodycamFPScomponent/Demo/Character/Anims/Anim_Arms_Pistol_Fire_Montage.Anim_Arms_Pistol_Fire_Montage"
    (:`then`
      (`SkeletalMeshComponent.PlayAnimation` (`self.Weapon`) "/Game/bodycamFPScomponent/Demo/Character/Anims/Anim_Pistol_Fire.Anim_Pistol_Fire" false))))

(fn `AimRot`
  (bind (_returnvalue_roll _returnvalue_pitch) (`KismetMathLibrary.BreakRotator` (`Controller.GetControlRotation` (`self.GetController`))))
  ;[1 1 1] エイムロット
  (if (or (`self.HasAuthority`) (`self.IsLocallyControlled`))
    (set `self.ControlRot_Rep` (`KismetMathLibrary.MakeRotator` 0.0 (* (`KismetMathLibrary.ClampAngle` _returnvalue_pitch 300.0 50.0) -1.0)))))

(fn `UserConstructionScript`)