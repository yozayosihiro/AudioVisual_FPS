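; Bodycam FPS camera component that adds movement-based camera shake and a moving vignette, with IsActive toggling post-process weight and effects.
; CameraShakeVignette optionally starts idle, walk or run shakes based on speed and the run flag.
; Clamped pitch and yaw deltas are smoothed with FInterpTo into the VignetteOffset parameter, making the vignette react to turning.
; While moving, interpolated random noise drives the VignetteShake parameter.
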(fn `Camera Shake & Vignette`
  (params (Camera :type "CameraComponent Object Reference") (Velocity :type "Vector Structure") (CameraRotation :type "Rotator Structure") (IsRun :type Boolean) (CameraShake :type Boolean) (IsActive :type Boolean))
  (bind _returnvalue (`GameplayStatics.GetPlayerController` 0))
  (bind (_camrotator_roll _camrotator_pitch _camrotator_yaw) (`KismetMathLibrary.BreakRotator` (`self.CamRotator`)))
  (bind _yawrateminmax (`self.YawRateMinMax`))
  (bind _pitchrateminmax (`self.PitchRateMinMax`))
  (bind _velocity (`self.Velocity`))
  (set `self.Camera` Camera)
  (set `self.Velocity` Velocity)
  (set `self.Camera Rotation` CameraRotation)
  (set `self.Camera Shake` CameraShake)
  (set `self.Is Running` IsRun)
  (set `CameraComponent.PostProcessBlendWeight` (`KismetMathLibrary.SelectFloat` 1.0 0.0 IsActive) (`self.Camera`))
  (if IsActive
    (`|ExecutionSequence`
      (:`then_0`
        (if (`self.Camera Shake`)
          ;[0 0 0] カメラの揺れ
          (if (< (`KismetMathLibrary.VSize` _velocity) 99.0)
            (`PlayerController.ClientStartCameraShake` :`self` _returnvalue :`Shake` "/Game/bodycamFPScomponent/Camera/CameraShake_Idle.CameraShake_Idle_C")
            (elif (> (`KismetMathLibrary.VSize` _velocity) 100.0)
              (if (`self.Is Running`)
                (`PlayerController.ClientStartCameraShake` :`self` _returnvalue :`Shake` "/Game/bodycamFPScomponent/Camera/CameraShake_Run.CameraShake_Run_C")
                (else
                  (`PlayerController.ClientStartCameraShake` :`self` _returnvalue :`Shake` "/Game/bodycamFPScomponent/Camera/CameraShake_Walk.CameraShake_Walk_C" :`Scale` 0.3)))))))
      (:`then_1`
        (set `self.PitchRate` (`KismetMathLibrary.FClamp` (+ (`self.PitchRate`) (- (.pitch (`self.Camera Rotation`)) _camrotator_pitch)) (* _pitchrateminmax -1.0) _pitchrateminmax))
        (set `self.YawRate` (`KismetMathLibrary.FClamp` (+ (`self.YawRate`) (- (.yaw (`self.Camera Rotation`)) _camrotator_yaw)) (* _yawrateminmax -1.0) _yawrateminmax))
        (set `self.CamRotator` (`self.Camera Rotation`))
        (bind _output_get (set `self.PitchVignetteOffset` (`KismetMathLibrary.FInterpTo` (`self.PitchVignetteOffset`) (`self.PitchRate`) (`GameplayStatics.GetWorldDeltaSeconds`) 10.0)))
        (bind _output_get_2 (set `self.YawVignetteOffset` (`KismetMathLibrary.FInterpTo` (`self.YawVignetteOffset`) (`self.YawRate`) (`GameplayStatics.GetWorldDeltaSeconds`) 10.0)))
        (`KismetMaterialLibrary.SetVectorParameterValue` null "VignetteOffset" (make `LinearColor` _output_get_2 _output_get 0.0 1.0))
        (set `self.YawRate` (`KismetMathLibrary.FInterpTo` 0.0 (`self.YawRate`) (`GameplayStatics.GetWorldDeltaSeconds`) 15.0))
        (set `self.PitchRate` (`KismetMathLibrary.FInterpTo` 0.0 (`self.PitchRate`) (`GameplayStatics.GetWorldDeltaSeconds`) 15.0)))
      (:`then_2`
        (if (> (`KismetMathLibrary.VSize` (`self.Velocity`)) 80.0)
          (set `self.PitchShake` (`KismetMathLibrary.FInterpTo` (`self.PitchShake`) (`KismetMathLibrary.RandomFloatInRange` -10.0 10.0) (`GameplayStatics.GetWorldDeltaSeconds`) 3.0))
          (set `self.YawShake` (`KismetMathLibrary.FInterpTo` (`self.YawShake`) (`KismetMathLibrary.RandomFloatInRange` -10.0 10.0) (`GameplayStatics.GetWorldDeltaSeconds`) 3.0))
          (bind _output_get_3 (set `self.PitchVignetteShake` (`KismetMathLibrary.FInterpTo` (`self.PitchVignetteShake`) (`self.PitchShake`) (`GameplayStatics.GetWorldDeltaSeconds`) 20.0)))
          (bind _output_get_4 (set `self.YawVignetteShake` (`KismetMathLibrary.FInterpTo` (`self.YawVignetteShake`) (`self.YawShake`) (`GameplayStatics.GetWorldDeltaSeconds`) 20.0)))
          (`KismetMaterialLibrary.SetVectorParameterValue` null "VignetteShake" (make `LinearColor` _output_get_4 _output_get_3 0.0 1.0))
          (set `self.PitchVignetteShake` (`KismetMathLibrary.FInterpTo` (`self.PitchShake`) 0.0 (`GameplayStatics.GetWorldDeltaSeconds`) 20.0))
          (set `self.YawVignetteShake` (`KismetMathLibrary.FInterpTo` (`self.YawShake`) 0.0 (`GameplayStatics.GetWorldDeltaSeconds`) 20.0)))))))