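; Base Blueprint for automatic firearms in the bodycam FPS kit, handling fire, inspect, melee and reload.
; Fire either loops through a Gate and retriggerable delay or runs one shot, per SemiOrFull, adding procedural recoil, effects, montages and a hit-scan.
; Melee reuses the hit-scan at short range after its montage.
; Reload waits out the empty or regular animation behind a DoOnce, then moves reserve ammo into the magazine.
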(event `self.Fire`
  (bind _playerref (`self.PlayerRef`))
  (bind _weapon_mesh (`self.Weapon_Mesh`))
  (bind _playerref_2 (`self.PlayerRef`))
  (bind _returnvalue (`SceneComponent.K2_GetComponentLocation` (`self.Weapon_Mesh`)))
  (bind _bp_ac_proceduralrecoil (`/Game/bodycamFPSkit/Blueprints/BP_FirstPersonCharacter.BP_AC_ProceduralRecoil` (`self.PlayerRef`)))
  ;[0 0 0] Fire Logic
  (if (and (not (`self.Reloading`)) (not (`self.IsInspect`)))
    (if (`/Game/bodycamFPSkit/Blueprints/BP_FirstPersonCharacter.IsRun` _playerref)
      (`/Game/bodycamFPSkit/Blueprints/BP_FirstPersonCharacter.StopRun` _playerref))
    (if (not (`self.IsFire`))
      (set `self.IsFire` true)
      (if (`self.SemiOrFull`)
        (`|ExecutionSequence`
          (:`then_0`
            (goto _label :!via `Open`))
          (:`then_1`
            (`/Engine/EditorBlueprintResources/StandardMacros.Gate` true :!label _label
              (:`Exit`
                (`|ExecutionSequence` :!label _label_2
                  (:`then_0`
                    (if (> (`self.AmmoCount`) 0)
                      (`/Game/bodycamFPSkit/Blueprints/BP_AC_ProceduralRecoil.Add Recoil` _bp_ac_proceduralrecoil (`self.RecoilValue`))
                      (bind _result (`/Engine/EditorBlueprintResources/StandardMacros.DecrementInt` (`self.AmmoCount`))
                        (:`  `
                          (set `self.AmmoCount` _result)
                          (`GameplayStatics.PlaySoundAtLocation` (`self.FireSound`) _returnvalue (struct) 1.0 1.0 0.0 null null null)
                          (`GameplayStatics.SpawnEmitterAttached` (`self.MuzzleFlash`) _weapon_mesh "muzzle" (0.0 0.0 0.0) (struct) (`self.MuzzleFlashScale`))
                          (`GameplayStatics.SpawnEmitterAttached` "/Game/bodycamFPSkit/ParticleEffects/P_MuzzleRing.P_MuzzleRing" _weapon_mesh "muzzle" (0.0 0.0 0.0) (struct) (`self.MuzzleRingScale`) "SnapToTarget")
                          (`self.SetWeaponAmmoData` false)
                          (`/Game/bodycamFPSkit/Character/AnimBP_FirstPersonCharacter.Recoil` (`/Game/bodycamFPSkit/Blueprints/BP_FirstPersonCharacter.AnimBP` _playerref_2))
                          (`|PlayMontage` (`/Game/bodycamFPSkit/Blueprints/BP_FirstPersonCharacter.Mesh1P` _playerref_2) (select `bool` (`/Game/bodycamFPSkit/Blueprints/BP_FirstPersonCharacter.AIM` (`self.PlayerRef`)) :`false` (`self.FireAnim`) :`true` (`self.ADSFireAnim`))
                            (:`then`
                              (`self.Fire_HitScan` false (`self.Range`)))
                            (:`OnBlendOut`
                              (if (== (`self.AmmoCount`) 0)
                                (`SkeletalMeshComponent.PlayAnimation` (`self.Weapon_Mesh`) (`self.EmptyWeaponAnim`) false))))))))
                  (:`then_1`
                    (`KismetSystemLibrary.RetriggerableDelay` (`self.FireDelay`))
                    (goto _label))
                  (:`then_2`
                    (if (== (`self.AmmoCount`) 0)
                      (`self.StopFire`)
                      (`/Game/bodycamFPSkit/Blueprints/BP_AC_ProceduralRecoil.Reset Recoil` _bp_ac_proceduralrecoil)
                      (`GameplayStatics.PlaySoundAtLocation` "/Game/bodycamFPSkit/Audio/Pistol_Audio/Sound_Pistol_DryFire.Sound_Pistol_DryFire" _returnvalue (struct) 1.0 1.0 0.0 null null null))))))))
        (else
          (goto _label_2))))))

(event `self.StopFire`
  ;[0 0 0] Fire Logic
  (set `self.IsFire` false)
  (`/Game/bodycamFPSkit/Blueprints/BP_AC_ProceduralRecoil.Reset Recoil` (`/Game/bodycamFPSkit/Blueprints/BP_FirstPersonCharacter.BP_AC_ProceduralRecoil` (`self.PlayerRef`)))
  (goto _label :!via `Close`))

(event `self.Inspect`
  ;[0 0 0] Inspect
  (if (and (not (`self.Reloading`)) (not (`self.IsInspect`)) (not (`/Game/bodycamFPSkit/Blueprints/BP_FirstPersonCharacter.AIM` (`self.PlayerRef`))) (not (`self.IsFire`)))
    (set `self.IsInspect` true)
    (`|PlayMontage` (`/Game/bodycamFPSkit/Blueprints/BP_FirstPersonCharacter.Mesh1P` (`self.PlayerRef`)) (`self.InspectAnim`)
      (:`OnCompleted`
        (set `self.IsInspect` false)))))

(event `self.Melee`
  ;[0 0 0] Melee
  (if (and (not (`self.Reloading`)) (not (`self.IsInspect`)) (not (`/Game/bodycamFPSkit/Blueprints/BP_FirstPersonCharacter.AIM` (`self.PlayerRef`))) (not (`self.IsFire`)))
    (`|PlayMontage` (`/Game/bodycamFPSkit/Blueprints/BP_FirstPersonCharacter.Mesh1P` (`self.PlayerRef`)) (`self.MeleeAnim`)
      (:`OnBlendOut`
        (`self.Fire_HitScan` false 250.0 "NewEnumerator0" true)))))

(event `self.Reload`
  (bind _reloadanim (`self.ReloadAnim`))
  (bind _emptyreloadanim (`self.EmptyReloadAnim`))
  (bind _returnvalue (- (`self.WeaponCapacity`) (`self.AmmoCount`)))
  (bind _animbp (`/Game/bodycamFPSkit/Blueprints/BP_FirstPersonCharacter.AnimBP` (`self.PlayerRef`)))
  ;[0 0 0] Reload
  (if (`self.IsFire`)
    _
    (elif (<= (`self.maxammo`) 0)
      _
      (elif (< (`self.AmmoCount`) (`self.WeaponCapacity`))
        (`/Engine/EditorBlueprintResources/StandardMacros.DoOnce` false :!label _label_3
          (:`Completed`
            (if (== (`self.AmmoCount`) 0)
              (`/Game/bodycamFPSkit/Character/AnimBP_FirstPersonCharacter.Reload` _animbp _emptyreloadanim 1)
              (`KismetSystemLibrary.Delay` (`AnimSequenceBase.SequenceLength` _emptyreloadanim))
              (else
                (`/Game/bodycamFPSkit/Character/AnimBP_FirstPersonCharacter.Reload` _animbp _reloadanim 1)
                (`KismetSystemLibrary.Delay` (`AnimSequenceBase.SequenceLength` _reloadanim))))
            (if (> (- (`self.WeaponCapacity`) (`self.AmmoCount`)) (`self.MaxAmmo`))
              (set `self.ammocount` (+ (`self.AmmoCount`) (`self.MaxAmmo`)))
              (set `self.maxammo` (- (`self.MaxAmmo`) (`self.MaxAmmo`)))
              (else
                (set `self.maxammo` (- (`self.MaxAmmo`) _returnvalue))
                (set `self.ammocount` (+ _returnvalue (`self.AmmoCount`)))))
            (`self.SetWeaponAmmoData` false)
            (`/Game/bodycamFPSkit/Character/AnimBP_FirstPersonCharacter.FinishReload` (`/Game/bodycamFPSkit/Blueprints/BP_FirstPersonCharacter.AnimBP` (`self.PlayerRef`)))
            (goto _label_3 :!via `Reset`)))))))

(fn `UserConstructionScript`
  (`parent.UserConstructionScript`))