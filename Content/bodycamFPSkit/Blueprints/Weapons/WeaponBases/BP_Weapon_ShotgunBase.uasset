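; Base shotgun weapon Blueprint for the bodycam FPS kit, handling firing, inspect, melee and reload.
; Fire spends ammo, plays effects, recoil and montages, then runs a shotgun hitscan; a delayed StopFire re-arms it.
; Reload chains begin, per-missing-shell loop and end animations through the player AnimBP, with ReloadBlendOut jumping to the end.
; Empty reloads temporarily swap the weapon's hand socket and suspend aiming.
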(event `self.Fire`
  (bind _weapon_mesh (`self.Weapon_Mesh`))
  (bind _playerref (`self.PlayerRef`))
  (bind _returnvalue (`SceneComponent.K2_GetComponentLocation` (`self.Weapon_Mesh`)))
  ;[0 0 0] Fire Logic
  (if (`self.Reloading`)
    _
    (elif (and (not (`self.Reloading`)) (not (`self.IsInspect`)))
      (if (`/Game/bodycamFPSkit/Blueprints/BP_FirstPersonCharacter.IsRun` _playerref)
        (`/Game/bodycamFPSkit/Blueprints/BP_FirstPersonCharacter.StopRun` _playerref))
      (if (not (`self.IsFire`))
        (set `self.IsFire` true)
        (`|ExecutionSequence`
          (:`then_0`
            (if (> (`self.AmmoCount`) 0)
              (`/Game/bodycamFPSkit/Blueprints/BP_AC_ProceduralRecoil.Add Recoil` (`/Game/bodycamFPSkit/Blueprints/BP_FirstPersonCharacter.BP_AC_ProceduralRecoil` (`self.PlayerRef`)) (`self.RecoilValue`))
              (bind _result (`/Engine/EditorBlueprintResources/StandardMacros.DecrementInt` (`self.AmmoCount`))
                (:`  `
                  (set `self.AmmoCount` _result)
                  (`GameplayStatics.PlaySoundAtLocation` (`self.FireSound`) _returnvalue (struct) 1.0 1.0 0.0 null null null)
                  (`GameplayStatics.SpawnEmitterAttached` (`self.MuzzleFlash`) _weapon_mesh "muzzle" (0.0 0.0 0.0) (struct) (`self.MuzzleFlashScale`))
                  (`GameplayStatics.SpawnEmitterAttached` "/Game/bodycamFPSkit/ParticleEffects/P_MuzzleRing.P_MuzzleRing" _weapon_mesh "muzzle" (0.0 0.0 0.0) (struct) (`self.MuzzleRingScale`) "SnapToTarget")
                  (`self.SetWeaponAmmoData` false)
                  (`/Game/bodycamFPSkit/Character/AnimBP_FirstPersonCharacter.Recoil` (`/Game/bodycamFPSkit/Blueprints/BP_FirstPersonCharacter.AnimBP` (`self.PlayerRef`)))
                  (`|PlayMontage` (`/Game/bodycamFPSkit/Blueprints/BP_FirstPersonCharacter.Mesh1P` (`self.PlayerRef`)) (select `bool` (`/Game/bodycamFPSkit/Blueprints/BP_FirstPersonCharacter.AIM` (`self.PlayerRef`)) :`false` (`self.FireAnim`) :`true` (`self.ADSFireAnim`))
                    (:`then`
                      (`self.Fire_HitScan` false (`self.Range`) "NewEnumerator7" false true)
                      (`/Game/bodycamFPSkit/Blueprints/BP_AC_ProceduralRecoil.Reset Recoil` (`/Game/bodycamFPSkit/Blueprints/BP_FirstPersonCharacter.BP_AC_ProceduralRecoil` (`self.PlayerRef`))))
                    (:`OnNotifyEnd`
                      (if (== (`self.AmmoCount`) 0)
                        (`SkeletalMeshComponent.PlayAnimation` (`self.Weapon_Mesh`) (`self.EmptyWeaponAnim`) false))))))))
          (:`then_1`
            (if (== (`self.AmmoCount`) 0)
              (`GameplayStatics.PlaySoundAtLocation` "/Game/bodycamFPSkit/Audio/Pistol_Audio/Sound_Pistol_DryFire.Sound_Pistol_DryFire" _returnvalue (struct) 1.0 1.0 0.0 null null null))))))))

(event `self.StopFire`
  ;[0 0 0] Fire Logic
  (`KismetSystemLibrary.Delay` 0.6)
  (set `self.IsFire` false))

(event `self.Inspect`
  ;[0 0 0] Inspect
  (if (and (not (`self.Reloading`)) (not (`self.IsInspect`)) (not (`/Game/bodycamFPSkit/Blueprints/BP_FirstPersonCharacter.AIM` (`self.PlayerRef`))) (not (`self.IsFire`)))
    (set `self.IsInspect` true)
    (`|PlayMontage` (`/Game/bodycamFPSkit/Blueprints/BP_FirstPersonCharacter.Mesh1P` (`self.PlayerRef`)) (`self.InspectAnim`)
      (:`OnCompleted`
        (set `self.IsInspect` false)))))

(event `self.Melee`
  ;[0 0 0] Melee
  (if (and (not (`self.Reloading`)) (not (`self.IsInspect`)) (not (`/Game/bodycamFPSkit/Blueprints/BP_FirstPersonCharacter.AIM` (`self.PlayerRef`))) (not (`self.IsFire`)))
    (`|PlayMontage` (`/Game/bodycamFPSkit/Blueprints/BP_FirstPersonCharacter.Mesh1P` (`self.PlayerRef`)) (`self.MeleeAnim`)
      (:`OnBlendOut`
        (`self.Fire_HitScan` false 250.0 "NewEnumerator0" true)))))

(event `self.Reload`
  (bind _reloademptybeginanim (`self.ReloadEmptyBeginAnim`))
  (bind _playerref (`self.PlayerRef`))
  (bind _playerref_2 (`self.PlayerRef`))
  (bind _playerref_3 (`self.PlayerRef`))
  (bind _reloademptybeginanim_2 (`self.ReloadEmptyBeginAnim`))
  (bind _playerref_4 (`self.PlayerRef`))
  (bind _playerref_5 (`self.PlayerRef`))
  (bind _playerref_6 (`self.PlayerRef`))
  (bind _returnvalue (- (`self.WeaponCapacity`) (`self.AmmoCount`)))
  ;[0 0 0] Reload
  (if (`self.IsFire`)
    _
    (elif (<= (`self.maxammo`) 0)
      _
      (elif (< (`self.AmmoCount`) (`self.WeaponCapacity`))
        (`/Engine/EditorBlueprintResources/StandardMacros.DoOnce` false :!label _label
          (:`Completed`
            (if (== (`self.AmmoCount`) 0)
              (set `/Game/bodycamFPSkit/Blueprints/BP_FirstPersonCharacter.CanAIM` false _playerref_6)
              (if (`/Game/bodycamFPSkit/Blueprints/BP_FirstPersonCharacter.AIM` _playerref_6)
                (`/Game/bodycamFPSkit/Blueprints/BP_FirstPersonCharacter.AIMOff` (`self.PlayerRef`))
                (`/Game/bodycamFPSkit/Blueprints/BP_FirstPersonCharacter.ChangeWeaponSocket` _playerref_3 true)
                (`/Game/bodycamFPSkit/Blueprints/BP_FirstPersonCharacter.SocketOffset` _playerref_3 (`self.Hand_L_SocketOffset`))
                (`/Game/bodycamFPSkit/Character/AnimBP_FirstPersonCharacter.Reload` (`/Game/bodycamFPSkit/Blueprints/BP_FirstPersonCharacter.AnimBP` _playerref_3) _reloademptybeginanim_2 1)
                (`KismetSystemLibrary.Delay` (`AnimSequenceBase.SequenceLength` _reloademptybeginanim_2))
                (`/Game/bodycamFPSkit/Blueprints/BP_FirstPersonCharacter.ChangeWeaponSocket` _playerref_4 false)
                (`/Game/bodycamFPSkit/Blueprints/BP_FirstPersonCharacter.SocketOffset` _playerref_4 (`self.Hand_R_SocketOffset`))
                (`/Game/bodycamFPSkit/Blueprints/BP_FirstPersonCharacter.AIMOn` _playerref_5)
                (else
                  (`/Game/bodycamFPSkit/Blueprints/BP_FirstPersonCharacter.ChangeWeaponSocket` _playerref_2 true)
                  (`/Game/bodycamFPSkit/Blueprints/BP_FirstPersonCharacter.SocketOffset` _playerref_2 (`self.Hand_L_SocketOffset`))
                  (`/Game/bodycamFPSkit/Character/AnimBP_FirstPersonCharacter.Reload` (`/Game/bodycamFPSkit/Blueprints/BP_FirstPersonCharacter.AnimBP` _playerref_2) _reloademptybeginanim 1)
                  (`KismetSystemLibrary.Delay` (`AnimSequenceBase.SequenceLength` _reloademptybeginanim))
                  (`/Game/bodycamFPSkit/Blueprints/BP_FirstPersonCharacter.ChangeWeaponSocket` _playerref false)
                  (`/Game/bodycamFPSkit/Blueprints/BP_FirstPersonCharacter.SocketOffset` _playerref (`self.Hand_R_SocketOffset`))))
              (set `/Game/bodycamFPSkit/Blueprints/BP_FirstPersonCharacter.CanAIM` true _playerref_5)
              (else
                (`/Game/bodycamFPSkit/Character/AnimBP_FirstPersonCharacter.Reload` (`/Game/bodycamFPSkit/Blueprints/BP_FirstPersonCharacter.AnimBP` (`self.PlayerRef`)) (`self.ReloadBeginAnim`) 1)))
            (`|ExecutionSequence`
              (:`then_0`
                (`/Game/bodycamFPSkit/Character/AnimBP_FirstPersonCharacter.Reload` (`/Game/bodycamFPSkit/Blueprints/BP_FirstPersonCharacter.AnimBP` (`self.PlayerRef`)) (`self.ReloadLoopAnim`) _returnvalue))
              (:`then_1`
                (`KismetSystemLibrary.RetriggerableDelay` (* _returnvalue (`AnimSequenceBase.SequenceLength` (`self.ReloadLoopAnim`))))
                (`/Game/bodycamFPSkit/Character/AnimBP_FirstPersonCharacter.Reload` (`/Game/bodycamFPSkit/Blueprints/BP_FirstPersonCharacter.AnimBP` (`self.PlayerRef`)) (`self.ReloadEndAnim`) 1 :!label _label_2)
                (`/Game/bodycamFPSkit/Character/AnimBP_FirstPersonCharacter.FinishReload` (`/Game/bodycamFPSkit/Blueprints/BP_FirstPersonCharacter.AnimBP` (`self.PlayerRef`)))
                (goto _label :!via `Reset`)))))))))

(event `ReloadBlendOut`
  ;[0 0 0] Reload
  (goto _label_2))

(fn `UserConstructionScript`
  (`parent.UserConstructionScript`))